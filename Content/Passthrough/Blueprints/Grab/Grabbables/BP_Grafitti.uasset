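; BP_Grafitti is a grabbable graffiti actor in the Passthrough content that snaps onto an anchor when released.
; When its GrabComponent fires OnDropped, it looks for BP_AnchorActor instances overlapping its StaticMesh.
; It moves to the first anchor's location and takes that anchor's rotation with a fixed 90-degree delta on every axis.
; With no overlap it stays put, and both outcomes print a debug message.
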(event OnDropped(GrabComponent)
  (bind _staticmesh (Variables|Default|GetStaticMesh))
  (bind _overlappingactors (Collision|GetOverlappingActors _staticmesh "/Game/Passthrough/Blueprints/BP_AnchorActor.BP_AnchorActor_C" :!class /Script/Engine.PrimitiveComponent))
  (bind _output (Utilities|Array|Get(acopy) _overlappingactors))
  (bind _returnvalue (Transformation|GetActorTransform _output))
  (if (> (Utilities|Array|Length _overlappingactors) 0)
    (Development|PrintString "Overlapping actors" true true "(R=0.000000,G=0.660000,B=1.000000,A=1.000000)" 2e+01)
    (Transformation|SetActorTransform (Math|Transform|MakeTransform (.location _returnvalue) (Math|Rotator|Delta(Rotator) (.rotation _returnvalue) "90.000000,90.000000,90.000000") "1.000000,1.000000,1.000000"))
    (else
      (Development|PrintString "No overlapping actors"))))

(event EventBeginPlay)

(fn ConstructionScript)