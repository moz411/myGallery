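; BP_Frame2 is a grabbable frame in the Passthrough project that snaps onto an anchor when released.
; When its GrabComponent fires OnDropped, it sphere-overlaps WorldStatic BP_AnchorActors within SphereRadius and takes the transform of a randomly picked one, with no empty-result check.
; Unconnected nodes that gather and sort anchor distances never run, so the snap is not to the nearest anchor.
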(event OnDropped(GrabComponent)
  (Development|PrintString "                                                                                      Dropped!")
  (bind _outactors (Collision|SphereOverlapActors (.location (Transformation|GetActorTransform self)) (Variables|Default|GetSphere%20Radius) (Utilities|Array|MakeArray "ObjectTypeQuery1") "/Game/Passthrough/Blueprints/BP_AnchorActor.BP_AnchorActor_C"))
  (Transformation|SetActorTransform (Transformation|GetActorTransform (.OutItem (Utilities|Array|Random _outactors)))))

(event EventBeginPlay)

(event Collision|EventActorBeginOverlap
  (params (OtherActor :type Actor%20Object%20Reference)))

(event EventTick
  (params (DeltaSeconds :type Float%20%28single-precision%29)))

(fn ConstructionScript)