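; Grabbable framed picture for passthrough that snaps onto a BP_Cross placement marker and saves its position as an Oculus spatial anchor.
; The construction script scales the frame from the picture plane's bounds and offsets the plane.
; Sphere overlap attaches the picture to the cross, creates and locally saves the anchor, then writes a newly created, unpopulated BP_SaveGallery to a save slot.
; Grabbing the picture detaches it.
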(event OnComponentBeginOverlap(Sphere)
  (params (OverlappedComponent :type Primitive%20Component%20Object%20Reference) (OtherActor :type Actor%20Object%20Reference) (OtherComp :type Primitive%20Component%20Object%20Reference) (OtherBodyIndex :type Integer) (bFromSweep :type Boolean) (SweepResult :type Hit%20Result%20Structure%20%28by%20ref%29))
  (bind _self self)
  (EventDispatchers|UnbindallEventsfromOnActorBeginOverlap)
  (Transformation|AttachActorToActor (Utilities|Array|Get(acopy) (Collision|GetOverlappingActors "/Game/Passthrough/Blueprints/BP_Cross.BP_Cross_C" :!class /Script/Engine.Actor)) "None" "SnapToTarget" "SnapToTarget" "KeepWorld" false)
  (|OculusXRAsyncCreateSpatialAnchor _self (Transformation|GetActorTransform _self)
    (:Success
      (|OculusXRAsyncSaveAnchor self "Local"
        (:then
          (bind _returnvalue (SaveGame|CreateSaveGameObject "/Game/Passthrough/Blueprints/BP_SaveGallery.BP_SaveGallery_C"))
          (|AsyncSaveGametoSlot _returnvalue (Variables|Default|GetSavegame)
            (:Completed
              (Development|PrintString "Anchors saved" true true "(R=0.000000,G=0.660000,B=1.000000,A=1.000000)" 2e+01))))))))

(event Custom|OnGrabbed_Event
  (Transformation|DetachFromActor "KeepRelative" "KeepRelative" "KeepRelative"))

(event EventBeginPlay
  (EventDispatchers|BindEventtoOnGrabbed (delegate Custom|OnGrabbed_Event)))

(fn ConstructionScript
  (bind _sm_plane (Variables|Default|GetSM_Plane))
  (bind _sm_frame (Variables|Default|GetSM_Frame))
  (bind (_min _max) (Components|StaticMesh|GetLocalBounds _sm_frame))
  (bind (_min_2 _max_2) (Components|StaticMesh|GetLocalBounds _sm_plane))
  ;[0.15 0.15 0.15 0.5] Scale frame
  (LocalVariables|SetBoxExtentContent (- _max_2 _min_2))
  (LocalVariables|SetBoxExtentFrame (- _max _min))
  (LocalVariables|SetScaleFactor (/ (LocalVariables|GetBoxExtentContent) (LocalVariables|GetBoxExtentFrame)))
  (Transformation|SetRelativeScale3D (Variables|Default|GetSM_Frame) (Math|Vector|MakeVector 2.0 (.y (+ (LocalVariables|GetScaleFactor) (Variables|/Script/Engine.SceneComponent|GetRelativeScale3D (Variables|Default|GetSM_Frame)))) (.z (+ (LocalVariables|GetScaleFactor) (Variables|/Script/Engine.SceneComponent|GetRelativeScale3D (Variables|Default|GetSM_Frame))))))
  (Transformation|AddLocalOffset (Variables|Default|GetSM_Plane) "-5.000000,0.000000,0.000000" false false))