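; BP_AnchorActor is an anchor in the Passthrough content, meant to snap overlapping actors to its own location and rotation.
; Its overlap handler moves only actors implementing BPI_AnchorActor, using a Locked flag against re-entry that stays set when any other actor triggers it.
; The node binding that handler to OnActorBeginOverlap is disconnected and BeginPlay is empty, so the Blueprint never binds it itself.
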(event Custom|OnActorBeginOverlap_Event
  (params (OverlappedActor :type Actor%20Object%20Reference) (OtherActor :type Actor%20Object%20Reference))
  (bind _self self)
  (bind _returnvalue (Transformation|GetActorTransform _self))
  (if (not (Variables|Default|Getlocked))
    (Variables|Default|Setlocked true)
    (if (Class|KismetSystemLibrary|DoesClassImplementInterface (Utilities|GetClass OtherActor) "/Game/Passthrough/Blueprints/BPI_AnchorActor.BPI_AnchorActor_C")
      (Transformation|SetActorLocationAndRotation OtherActor (.location _returnvalue) (.rotation _returnvalue))
      (Variables|Default|Setlocked false))))

(event EventBeginPlay)

(fn ConstructionScript)